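; BP_SituationCard is a card actor that shows a Description as wrapped text on a TextRender component.
; The Construction Script runs WrapText and sets the result on the component.
; WrapText splits the string into pieces and rejoins them, inserting <br> tags when the running character count exceeds CharactersPerLine.
; BeginPlay repeats the wrap but leaves the result unused, as its SetText and print nodes are disconnected.
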(event `self.ReceiveBeginPlay`
  (bind _wrapedtext (`self.WrapText` (`self.Description`) (`self.Characters per line`))))

(event `self.ReceiveTick`
  (params (DeltaSeconds :type "Float (single-precision)")))

(fn `UserConstructionScript`
  (bind _wrapedtext (`self.WrapText` (`self.Description`) (`self.Characters per line`)))
  (`TextRenderComponent.K2_SetText` (`self.TextRender`) _wrapedtext))

(fn `WrapText`
  (params (Text :type Text) (`Characters per line` :type Integer))
  (returns (WrapedText :type Text))
  (locals (FinalText :type Text) (CharacterCount :type Integer))
  (set `local.CharacterCount` 0)
  (for _array_element (`KismetStringLibrary.ParseIntoArray` (`KismetTextLibrary.Conv_TextToString` Text))
    (bind _output_get (set `local.CharacterCount` (+ (`KismetStringLibrary.Len` _array_element) (`local.CharacterCount`))))
    (if (> _output_get `Characters per line`)
      (set `local.FinalText` (`|FormatText` "{0}<br> {1}" (`local.FinalText`) _array_element))
      (set `local.CharacterCount` 0)
      (else
        (set `local.FinalText` (`|FormatText` "{0} {1}" (`local.FinalText`) _array_element)))))
  (return (`local.FinalText`)))