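; Game mode that runs a turn-based card game, tracking Money, Followers, Power and Vigilence until a win or lose level opens.
; Each turn it draws a situation card and spawns action cards matching its tag; choosing one starts the next turn.
; Cards apply timed stat modifiers, queue temporary consequence cards and toggle data-table card sets.
; Draws are weighted random, using cumulative probabilities from base weights and current stats scaled by multipliers.
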(event `Turn begun`
  (bind _card_set (`self.Card Set`))
  (bind (_money _followers _power _vigilence) (break `/Game/Datas/F_GameStats` (`self.Game stats`)))
  ;[1 1 1] Récupération des cartes de début de partie
  (if (>= _money 1000)
    (`GameplayStatics.OpenLevel` "EndingWin" :!label _label)
    (elif (>= _followers 30)
      (goto _label)
      (elif (>= _power 100)
        (goto _label)
        (elif (<= _money 0)
          (`GameplayStatics.OpenLevel` "EndingLose" :!label _label_2)
          (elif (>= _vigilence 100)
            (goto _label_2)
            (else
              (`/Engine/EditorBlueprintResources/StandardMacros.IncrementInt` (`self.Turn`)
                (:`  `
                  (`self.Update Temporary Cards`)
                  (`self.Update Stat Modifiers`)
                  (bind _drawn_cards (`self.Draw Cards From Type And Tag` _card_set "NewEnumerator0" (struct :`TagName` "Base") 1))
                  (bind _output (`|GetArrayItem` _drawn_cards))
                  (bind ((`ID_55_681B341A4613154C989696910D32D2A3` _id) (`Tag_11_2934B09947F65A88514175896BA33A24` _tag) (`Consequencescards_56_D13B4EAE4484026F9AC8B4A6A9D4707A` _consequencescards) (`StatModifiers_54_DAD43CEB4E460537F2F10C9A635A4E17` _statmodifiers) (`UnlockLockCardSet_50_2350D422486E3A0F3D662382CA607D6F` _unlocklockcardset)) (break `/Game/Datas/F_Card` _output))
                  (`self.Add Stat Modifiers` _statmodifiers)
                  (`self.Apply Stats Modifiers` "NewEnumerator0")
                  (`self.Apply Stats Modifiers` "NewEnumerator2")
                  (`self.Add Consequences Cards` _consequencescards)
                  (`/Engine/EditorBlueprintResources/StandardMacros.IsValid` _unlocklockcardset
                    (:`Is Valid`
                      (bind _card_set_2 (`self.Get Card Set` _unlocklockcardset))
                      (`KismetArrayLibrary.Array_Append` (`self.Card Set`) _card_set_2))
                    (:`Is Not Valid`
                      _))
                  (`self.Situation Card Drawn` _output)
                  (bind _drawn_cards_2 (`self.Draw Cards From Type And Tag` _card_set "NewEnumerator1" _tag (`self.Action Card Count`)))
                  (`self.Action Card Drawn` _drawn_cards_2))))))))))

(event `self.ReceiveBeginPlay`
  (set `self.Game stats` (make `/Game/Datas/F_GameStats` 500 3))
  (bind _card_set (`self.Get Card Set` "/Game/Datas/DT_BasicCards.DT_BasicCards"))
  (set `self.Card Set` _card_set)
  (set `self.Turn` 0)
  (`KismetSystemLibrary.PrintString` (`KismetSystemLibrary.GetDisplayName` (`self.SituationSpawner`))))

(event `Game Ready`
  (`self.Turn begun`))

(event `Situation Card Drawn`
  (params (Card :type "/Game/Datas/F_Card Structure"))
  (bind _situationcard (`self.SituationCard`))
  (`/Engine/EditorBlueprintResources/StandardMacros.IsValid` _situationcard
    (:`Is Valid`
      (`self.K2_DestroyActor` _situationcard))
    (:`Is Not Valid`
      _))
  (bind _returnvalue (`|SpawnActorFromClass` "/Game/Blueprints/BP_SituationCard.BP_SituationCard_C" (`KismetMathLibrary.MakeTransform` (`self.K2_GetActorLocation` (`self.SituationSpawner`)) (struct :`Yaw` 90.0) (0.7 0.7 0.7)) "Undefined" "OverrideRootScale" null (`.Description_5_28664E6049D95DB37A53C4B70C73F96D` (break `/Game/Datas/F_Card` Card)) null))
  (set `self.SituationCard` _returnvalue))

(event `Action card chosen`
  (params (Card :type "/Game/Datas/F_Card Structure"))
  (bind ((`ID_55_681B341A4613154C989696910D32D2A3` _id) (`Consequencescards_56_D13B4EAE4484026F9AC8B4A6A9D4707A` _consequencescards) (`StatModifiers_54_DAD43CEB4E460537F2F10C9A635A4E17` _statmodifiers) (`UnlockLockCardSet_50_2350D422486E3A0F3D662382CA607D6F` _unlocklockcardset)) (break `/Game/Datas/F_Card` Card))
  (`GameplayStatics.PlaySound2D` "/Game/Sounds/CardSwipe.CardSwipe" 1.0 1.0 0.0 null null)
  (`self.Add Stat Modifiers` _statmodifiers "NewEnumerator1")
  (`self.Apply Stats Modifiers` "NewEnumerator1")
  (`self.Add Consequences Cards` _consequencescards)
  (`/Engine/EditorBlueprintResources/StandardMacros.IsValid` _unlocklockcardset
    (:`Is Valid`
      (bind _card_set (`self.Get Card Set` _unlocklockcardset))
      (`KismetArrayLibrary.Array_Append` (`self.Card Set`) _card_set))
    (:`Is Not Valid`
      _))
  (`self.Turn begun`))

(event `Action Card Drawn`
  (params (Cards :type "Array of /Game/Datas/F_Card Structure"))
  (bind _actioncards (`self.ActionCards`))
  (for _array_element _actioncards
    (`self.K2_DestroyActor` _array_element))
  (`KismetArrayLibrary.Array_Clear` _actioncards)
  (for (_array_element_2 _array_index) Cards
    (if (== (mod (`KismetArrayLibrary.Array_Length` Cards) 2) 0)
      (bind _returnvalue (`|SpawnActorFromClass` "/Game/Blueprints/BP_ActionCard.BP_ActionCard_C" (`KismetMathLibrary.MakeTransform` (`self.K2_GetActorLocation` (`|GetArrayItem` (`self.EvenSpawners`) _array_index)) (struct :`Yaw` 90.0) (0.4 0.4 0.4)) "Undefined" "OverrideRootScale" null _array_element_2 null))
      (`KismetArrayLibrary.Array_Add` (`self.ActionCards`) _returnvalue)
      (else
        (bind _returnvalue_2 (`|SpawnActorFromClass` "/Game/Blueprints/BP_ActionCard.BP_ActionCard_C" (`KismetMathLibrary.MakeTransform` (`self.K2_GetActorLocation` (`|GetArrayItem` (`self.OddSpawners`) _array_index)) (struct :`Yaw` 90.0) (0.4 0.4 0.4)) "Undefined" "OverrideRootScale" null _array_element_2 null))
        (`KismetArrayLibrary.Array_Add` (`self.ActionCards`) _returnvalue_2)))))

(fn `Add Consequences Cards`
  (params (`Cards to add` :type "Array of Name"))
  (for _array_element `Cards to add`
    (for _array_element_2 (`self.Card Set`)
      (if (== (`.ID_55_681B341A4613154C989696910D32D2A3` (break `/Game/Datas/F_Card` _array_element_2)) _array_element)
        (bind _structout (setmembers `/Game/Datas/F_Card` :`StructRef` _array_element_2 :`Add Turn` (`self.Turn`)))
        (`KismetArrayLibrary.Array_Add` (`self.TemporaryCards`) _structout)
        (break))))
  (return))

(fn `Add Stat Modifiers`
  (params (Modifiers :type "Array of /Game/Datas/F_StatModifier Structure") (`Card type` :type "/Game/Datas/E_CardType Enum" :default "NewEnumerator0"))
  (for (_array_element _array_index) Modifiers
    (bind _structout (setmembers `/Game/Datas/F_StatModifier` :`StructRef` _array_element :`Card type` `Card type`))
    (`KismetArrayLibrary.Array_Set` Modifiers _array_index _structout))
  (`KismetArrayLibrary.Array_Append` (`self.Stats Modifiers`) Modifiers)
  (return))

(fn `Apply Stats Modifiers`
  (params (Type :type "/Game/Datas/E_CardType Enum" :default "NewEnumerator0"))
  (locals (MoneyModif :type Integer) (FollowersModif :type Integer) (PowerModif :type Integer) (VigilenceModif :type Integer) (ActionCountModif :type Integer))
  (bind _game_stats (`self.Game stats`))
  (bind (_money _followers _power _vigilence) (break `/Game/Datas/F_GameStats` _game_stats))
  (for _array_element (`self.Stats Modifiers`)
    (bind ((`StatName_3_1650DDA44C1736A1F8F108A8ED2F4DAA` _statname) (`Cardtype_13_81374669420FC7AC587ED28B567A64DB` _cardtype)) (break `/Game/Datas/F_StatModifier` _array_element))
    (if (`|EnumEquality` _cardtype Type)
      (switch `name` _statname
        (:`Money`
          (bind ((`Value_10_883BD72749B855EDEF0DA4A08DEF68C3` _value)) (break `/Game/Datas/F_StatModifier` _array_element))
          (set `local.MoneyModif` (+ (`local.MoneyModif`) _value)))
        (:`Followers`
          (set `local.FollowersModif` (+ (`local.FollowersModif`) _value)))
        (:`Power`
          (set `local.PowerModif` (+ (`local.PowerModif`) _value)))
        (:`Vigilence`
          (set `local.VigilenceModif` (+ (`local.VigilenceModif`) _value)))
        (:`Action Count`
          (set `local.ActionCountModif` (+ (`local.ActionCountModif`) _value))))))
  (setmembers `/Game/Datas/F_GameStats` :`StructRef` _game_stats :`Money` (+ _money (`local.MoneyModif`)) :`Followers` (+ (`local.FollowersModif`) _followers) :`Power` (+ (`local.PowerModif`) _power) :`Vigilence` (+ (`local.VigilenceModif`) _vigilence))
  (set `self.Action Card Count` (+ (`local.ActionCountModif`) (`self.Action Card Count`)))
  (return))

(fn `Compute Cards Probabilities`
  (params (`Cards to compute` :type "Array of /Game/Datas/F_Card Structure"))
  (returns (`Proba List1` :type "Array of /Game/Datas/F_Probability Structure"))
  (locals (TotalWeight :type Integer) (Cards :type "Array of /Game/Datas/F_Card Structure") (`Proba List` :type "Array of /Game/Datas/F_Probability Structure"))
  (bind _proba_list (`local.Proba List`))
  ;[1 1 1] Calcul du poids total
  (bind _output_get (set `local.Cards` `Cards to compute`))
  (for _array_element _output_get
    (set `local.TotalWeight` (+ (`local.TotalWeight`) (`.CurrentWeight_31_60724458456DB220D675E2AC690EB2C3` (break `/Game/Datas/F_Card` _array_element)))))
  ;[1 1 1] Calcul des probas d'apparition pour chaque carte en fonction de son poids
  (for (_array_element_2 _array_index) _output_get
    (if (== (`KismetArrayLibrary.Array_Length` _proba_list) 0)
      (bind _returnvalue (* (`KismetMathLibrary.SafeDivide` (`KismetMathLibrary.Conv_IntToDouble` (`.CurrentWeight_31_60724458456DB220D675E2AC690EB2C3` (break `/Game/Datas/F_Card` _array_element_2))) (`KismetMathLibrary.Conv_IntToDouble` (`local.TotalWeight`))) 100.0))
      (`KismetArrayLibrary.Array_Add` (`local.Proba List`) (make `/Game/Datas/F_Probability` _array_index _returnvalue))
      (else
        (`KismetArrayLibrary.Array_Add` (`local.Proba List`) (make `/Game/Datas/F_Probability` _array_index (+ _returnvalue (`.Probability_5_67E924E544DD44E481242A89F6D842B1` (break `/Game/Datas/F_Probability` (`|GetArrayItem` _proba_list (`KismetArrayLibrary.Array_LastIndex` _proba_list))))))))))
  (return (`local.Proba List`)))

(fn `Compute Cards Weight`
  (params (`Cards to Compute` :type "Array of /Game/Datas/F_Card Structure"))
  (returns (`Cards computed` :type "Array of /Game/Datas/F_Card Structure"))
  (locals (Cards :type "Array of /Game/Datas/F_Card Structure"))
  (bind _stats_multipliers (`self.Stats Multipliers`))
  (bind (_game_stats_money _game_stats_followers _game_stats_power _game_stats_vigilence) (break `/Game/Datas/F_GameStats` (`self.Game stats`)))
  (bind _output_get (set `local.Cards` `Cards to Compute`))
  (for (_array_element _array_index) _output_get
    (bind ((`ID_55_681B341A4613154C989696910D32D2A3` _id) (`Statsinfluence_27_A5D72FA846077349921F959101BC70A9` _statsinfluence) (`BaseWaight_28_543523BE4BDD57C4EAB76A8BE459B67E` _basewaight)) (break `/Game/Datas/F_Card` _array_element))
    (bind (_money _followers _power _vigilence) (break `/Game/Datas/F_GameStats` _statsinfluence))
    ;[1 1 1] On recalcule le poids de la carte en fonction de l'influence de chaque stats et des stats du jeu
    (bind _structout (setmembers `/Game/Datas/F_Card` :`StructRef` _array_element :`Current Weight` (`KismetMathLibrary.Clamp` (`KismetMathLibrary.FTrunc` (+ (`KismetMathLibrary.Conv_IntToDouble` _basewaight) (* (* (`KismetMathLibrary.Conv_IntToDouble` _money) (`/Game/Blueprints/Data/DA_StatsMultipliers.Money Multiplier` _stats_multipliers)) (`KismetMathLibrary.Conv_IntToDouble` _game_stats_money)) (* (* (`KismetMathLibrary.Conv_IntToDouble` _followers) (`/Game/Blueprints/Data/DA_StatsMultipliers.Followers Multiplier` _stats_multipliers)) (`KismetMathLibrary.Conv_IntToDouble` _game_stats_followers)) (* (* (`KismetMathLibrary.Conv_IntToDouble` _power) (`/Game/Blueprints/Data/DA_StatsMultipliers.Power Multiplier` _stats_multipliers)) (`KismetMathLibrary.Conv_IntToDouble` _game_stats_power)) (* (* (`KismetMathLibrary.Conv_IntToDouble` _vigilence) (`/Game/Blueprints/Data/DA_StatsMultipliers.Vigilence Multiplier` _stats_multipliers)) (`KismetMathLibrary.Conv_IntToDouble` _game_stats_vigilence)))) 1 1000000000)))
    (`KismetArrayLibrary.Array_Set` (`local.Cards`) _array_index _structout))
  (return (`local.Cards`)))

(fn `Draw Cards`
  (params (`Number of cards to draw` :type Integer) (`Proba List` :type "Array of /Game/Datas/F_Probability Structure"))
  (returns (`Drawn Cards` :type "Array of Integer"))
  (locals (Cards :type "Array of Integer") (`List Proba` :type "Array of /Game/Datas/F_Probability Structure") (RandomValue :type "Float (double-precision)") (DrawnCard :type Integer :default -1) (NbCardToDraw :type Integer))
  (bind _returnvalue (`KismetArrayLibrary.Array_Length` `Proba List`))
  (bind _drawncard (`local.DrawnCard`))
  (if (< `Number of cards to draw` _returnvalue)
    (set `local.NbCardToDraw` `Number of cards to draw`)
    (else
      ;[1 1 1] On boucle sur le nombre de carte à tirer, on tire un nombre aléatoire
      (set `local.NbCardToDraw` _returnvalue)))
  (set `local.List Proba` `Proba List`)
  (for _ (range 1 (+ (`local.NbCardToDraw`) 1))
    (while (or (== _drawncard -1) (!= (`KismetArrayLibrary.Array_Find` (`local.Cards`) _drawncard) -1))
      (set `local.RandomValue` (`KismetMathLibrary.RandomFloatInRange` 0.0 100.0))
      ;[1 1 1] On cherche la 1ère carte dont la proba est supérieure à la proba tirée
      (for _index (range (+ (`KismetArrayLibrary.Array_Length` `Proba List`) 1))
        (bind (_cardid _probability) (break `/Game/Datas/F_Probability` (`|GetArrayItem` (`local.List Proba`) _index)))
        (if (<= (`local.RandomValue`) _probability)
          (set `local.DrawnCard` _cardid)
          (break))))
    (`KismetArrayLibrary.Array_Add` (`local.Cards`) (`local.DrawnCard`)))
  (return (`local.Cards`)))

(fn `Draw Cards From Type And Tag`
  (params (Cards :type "Array of /Game/Datas/F_Card Structure") (`Card Type` :type "/Game/Datas/E_CardType Enum" :default "NewEnumerator0") (Tag :type "GameplayTag Structure") (`Number of cards to draw` :type Integer))
  (returns (`Drawn Cards` :type "Array of /Game/Datas/F_Card Structure"))
  (locals (DrawnCards :type "Array of /Game/Datas/F_Card Structure") (TempCardSet :type "Array of /Game/Datas/F_Card Structure"))
  (bind _card_set (`self.Card Set`))
  (bind _card_set_2 (`self.Card Set`))
  (bind _filtered_cards (`self.Filter Card Set` `Card Type` Cards Tag))
  (if (`|EnumEquality` `Card Type` "NewEnumerator0")
    (`KismetArrayLibrary.Array_Append` _filtered_cards (`self.TemporaryCards`)))
  (bind _cards_computed (`self.Compute Cards Weight` _filtered_cards))
  (bind _proba_list1 (`self.Compute Cards Probabilities` _cards_computed))
  (bind _drawn_cards (`self.Draw Cards` `Number of cards to draw` _proba_list1))
  (for _array_element _drawn_cards
    (bind _output (`|GetArrayItem` _cards_computed _array_element))
    (`KismetArrayLibrary.Array_Add` (`local.DrawnCards`) _output)
    (bind ((`ID_55_681B341A4613154C989696910D32D2A3` _id) (`Cardtype_2_953E406140982E354CF8C19AFBFB7424` _cardtype) (`Consequencescards_56_D13B4EAE4484026F9AC8B4A6A9D4707A` _consequencescards) (`StatModifiers_54_DAD43CEB4E460537F2F10C9A635A4E17` _statmodifiers) (`UnlockLockCardSet_50_2350D422486E3A0F3D662382CA607D6F` _unlocklockcardset) (`AddTurn_38_EDA4D32A4EDAE8B0485E539C9C074BF1` _addturn) (`Unique?_41_7D19B933409DC81FEBED3B923AB1C999` _unique_)) (break `/Game/Datas/F_Card` _output))
    ;[1 1 1] Si la carte tirée est un carte de conséquences, on supprime toutes les cartes tirées au même tour des cartes temporaires (car une seule conséquence est possible)
    (if (`|EnumEquality` _cardtype "NewEnumerator2")
      (`self.Remove Temporary Cards Of Turn` _addturn)
      (if _unique_
        (bind _output_get (set `local.TempCardSet` _card_set_2))
        (for _array_element_2 _output_get
          (if (== (`.ID_55_681B341A4613154C989696910D32D2A3` (break `/Game/Datas/F_Card` _array_element_2)) _id)
            (`KismetArrayLibrary.Array_RemoveItem` _card_set_2 _array_element_2))))
      (elif _unique_
        (for _array_element_3 _card_set
          (if (== (`.ID_55_681B341A4613154C989696910D32D2A3` (break `/Game/Datas/F_Card` _array_element_3)) _id)
            (`KismetArrayLibrary.Array_RemoveItem` _card_set _array_element_3))))))
  (return (`local.DrawnCards`)))

(fn `Filter Card Set`
  (params (`Card Type` :type "/Game/Datas/E_CardType Enum" :default "NewEnumerator0") (Cards :type "Array of /Game/Datas/F_Card Structure") (Tag :type "GameplayTag Structure"))
  (returns (`Filtered Cards` :type "Array of /Game/Datas/F_Card Structure"))
  (locals (FilteredCards :type "Array of /Game/Datas/F_Card Structure"))
  (for _array_element Cards
    (bind ((`ID_55_681B341A4613154C989696910D32D2A3` _id) (`Cardtype_2_953E406140982E354CF8C19AFBFB7424` _cardtype) (`Tag_11_2934B09947F65A88514175896BA33A24` _tag)) (break `/Game/Datas/F_Card` _array_element))
    (if (and (`|EnumEquality` _cardtype `Card Type`) (`BlueprintGameplayTagLibrary.MatchesTag` _tag Tag (`|EnumEquality` `Card Type` "NewEnumerator1")))
      (`KismetArrayLibrary.Array_Add` (`local.FilteredCards`) _array_element)))
  (return (`local.FilteredCards`)))

(fn `Get Card Set`
  (params (`Cards Data Table` :type "DataTable Object Reference"))
  (returns (`Card Set` :type "Array of /Game/Datas/F_Card Structure"))
  (locals (Cards :type "Array of /Game/Datas/F_Card Structure"))
  (bind _card_set (`self.Card Set`))
  (if (`KismetArrayLibrary.Array_Contains` (`self.CardSetAdded`) `Cards Data Table`)
    (bind _outrownames (`DataTableFunctionLibrary.GetDataTableRowNames` `Cards Data Table`))
    (for _array_element _outrownames
      (bind _returnvalue (`|GetDataTableRow` `Cards Data Table` _array_element)
        (:`then`
          (for _array_element_2 _card_set
            (if (== (`.ID_55_681B341A4613154C989696910D32D2A3` (break `/Game/Datas/F_Card` _array_element_2)) (`.ID_55_681B341A4613154C989696910D32D2A3` (break `/Game/Datas/F_Card` _returnvalue)))
              (`KismetArrayLibrary.Array_RemoveItem` _card_set _array_element_2))))))
    (return)
    (else
      ;[1 1 1] On ajoute les cartes si elles n'ont pas déjà été ajoutées
      (`KismetArrayLibrary.Array_Add` (`self.CardSetAdded`) `Cards Data Table`)
      (bind _outrownames_2 (`DataTableFunctionLibrary.GetDataTableRowNames` `Cards Data Table`))
      (for _array_element_3 _outrownames_2
        (bind _returnvalue_2 (`|GetDataTableRow` `Cards Data Table` _array_element_3)
          (:`then`
            (`KismetArrayLibrary.Array_Add` (`local.Cards`) _returnvalue_2))))
      (return (`local.Cards`)))))

(fn `Remove Temporary Cards Of Turn`
  (params (Turn :type Integer))
  (locals (TempTemp :type "Array of /Game/Datas/F_Card Structure"))
  (bind _output_get (set `local.TempTemp` (`self.TemporaryCards`)))
  (for _array_element _output_get
    (if (== Turn (`.AddTurn_38_EDA4D32A4EDAE8B0485E539C9C074BF1` (break `/Game/Datas/F_Card` _array_element)))
      (`KismetArrayLibrary.Array_RemoveItem` (`self.TemporaryCards`) _array_element)))
  (return))

(fn `Update Stat Modifiers`
  (locals (tempModifiers :type "Array of /Game/Datas/F_StatModifier Structure"))
  (bind _stats_modifiers (`self.Stats Modifiers`))
  ;[1 1 1] Maj du nombre de tour passé pour chaque modifieurs
  (for (_array_element _array_index) _stats_modifiers
    (bind _structout (setmembers `/Game/Datas/F_StatModifier` :`StructRef` _array_element :`Tour Passed` (+ (`.TourPassed_7_756AA71B4D723608AA4ED7A8AABE0466` (break `/Game/Datas/F_StatModifier` _array_element)) 1)))
    (`KismetArrayLibrary.Array_Set` _stats_modifiers _array_index _structout))
  ;[1 1 1] Suppression modifieurs si nombre de tour passé supérieur au nombre de tour max
  (bind _output_get (set `local.tempModifiers` _stats_modifiers))
  (for _array_element_2 _output_get
    (bind ((`TourPresence_8_57DAB73143F30B82FD10EBAB6D4BD522` _tourpresence) (`TourPassed_7_756AA71B4D723608AA4ED7A8AABE0466` _tourpassed)) (break `/Game/Datas/F_StatModifier` _array_element_2))
    (if (>= _tourpassed _tourpresence)
      (`KismetArrayLibrary.Array_RemoveItem` (`self.Stats Modifiers`) _array_element_2)))
  (return))

(fn `Update Temporary Cards`
  (bind _temporarycards (`self.TemporaryCards`))
  (for (_array_element _array_index) _temporarycards
    (bind ((`ID_55_681B341A4613154C989696910D32D2A3` _id) (`Tourpresence_18_7610AF074FDBC33DD662C7AA1B1463BC` _tourpresence) (`Passedtours_17_6F12FA1D4D7025BBCAB32087DFDAA595` _passedtours)) (break `/Game/Datas/F_Card` _array_element))
    (if (>= _passedtours _tourpresence)
      (`KismetArrayLibrary.Array_Remove` _temporarycards _array_index)
      (else
        (bind _structout (setmembers `/Game/Datas/F_Card` :`StructRef` _array_element :`Passed tours` (+ _passedtours 1)))
        (`KismetArrayLibrary.Array_Set` _temporarycards _array_index _structout))))
  (return))

(fn `UserConstructionScript`)