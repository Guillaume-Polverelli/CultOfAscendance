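; Clickable action card actor that can be hovered, dragged, and played, showing its wrapped description on a paper sprite.
; Hover enlarges and nudges it, guarded by a shared PC_Main flag; clicking toggles dragging along Y/Z via cursor traces.
; On release, Tick timeline-lerps it back to its start unless PlayCard is set, in which case a dynamic-material dissolve runs, then reports the card to GM_Main.
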(event `OnBeginCursorOver_Event` :!signature `self.OnBeginCursorOver`
  (params (TouchedActor :type "Actor Object Reference"))
  (bind _aspc_main (cast `/Game/Blueprints/PC_Main` (`GameplayStatics.GetPlayerController` 0)))
  (if (not (`/Game/Blueprints/PC_Main.bHoverCard` _aspc_main))
    (`self.SetActorScale3D` (0.45 0.45 0.45))
    (`self.K2_SetActorLocation` (`KismetMathLibrary.MakeVector` (+ (.x (`self.StartLocation`)) -30.0) (.y (`self.StartLocation`)) (.z (`self.StartLocation`))) false true)
    (set `/Game/Blueprints/PC_Main.bHoverCard` true _aspc_main)))

(event `OnEndCursorOver_Event` :!signature `self.OnEndCursorOver`
  (params (TouchedActor :type "Actor Object Reference"))
  (`self.SetActorScale3D` (0.4 0.4 0.4))
  (`self.K2_SetActorLocation` (`self.StartLocation`) false true)
  (bind _aspc_main (cast `/Game/Blueprints/PC_Main` (`GameplayStatics.GetPlayerController` 0)))
  (set `/Game/Blueprints/PC_Main.bHoverCard` false _aspc_main))

(event `self.ReceiveBeginPlay`
  (set `self.StartLocation` (`self.K2_GetActorLocation`))
  (add `self.OnClicked` (delegate `OnClicked_Event`))
  (add `self.OnBeginCursorOver` (delegate `OnBeginCursorOver_Event`))
  (add `self.OnEndCursorOver` (delegate `OnEndCursorOver_Event`))
  (add `self.ReturnInitialPositionDelegate` (delegate `ReturnToInitialPosition`)))

(event `OnClicked_Event` :!signature `self.OnClicked`
  (params (TouchedActor :type "Actor Object Reference") (ButtonPressed :type "Key Structure" :default "None"))
  (set `self.bDrag` (not (`self.bDrag`))))

(event `ReturnToInitialPosition`
  (set `self.bAnimation` true)
  (set `self.CurrentLoc` (`self.K2_GetActorLocation`))
  (bind (_direction _position) (`Timeline|Timeline` :!via `PlayFromStart`)
    (:`Update`
      (`self.K2_SetActorLocation` (`KismetMathLibrary.VLerp` (`self.CurrentLoc`) (`self.StartLocation`) _position)))
    (:`Finished`
      (`self.ResetReturnToLoc`)
      (set `self.bAnimation` false))))

(event `self.ReceiveTick`
  (params (DeltaSeconds :type "Float (single-precision)"))
  (bind _y (.y (`self.K2_GetActorLocation`)))
  (bind _z (.z (`self.K2_GetActorLocation`)))
  (bind _y_2 (.y (`self.StartLocation`)))
  (bind _z_2 (.z (`self.StartLocation`)))
  (if (`self.bDrag`)
    (`self.K2_SetActorLocation` self (`KismetMathLibrary.MakeVector` (.x (`self.K2_GetActorLocation` self)) (.y (`.Location` (`GameplayStatics.BreakHitResult` (`PlayerController.GetHitResultUnderCursorByChannel` (`GameplayStatics.GetPlayerController` 0) "TraceTypeQuery1" true)))) (.z (`.Location` (`GameplayStatics.BreakHitResult` (`PlayerController.GetHitResultUnderCursorByChannel` (`GameplayStatics.GetPlayerController` 0) "TraceTypeQuery1" true))))) true false)
    (elif (and (`self.bPlayCard`) (not (`self.bAnimation`)))
      (`/Engine/EditorBlueprintResources/StandardMacros.DoOnce` false
        (:`Completed`
          (bind _aspc_main (cast `/Game/Blueprints/PC_Main` (`GameplayStatics.GetPlayerController` 0)))
          (set `/Game/Blueprints/PC_Main.bHoverCard` false _aspc_main)
          (`self.PlayDisolveAnimation`)))
      (elif (and (or (> _y (+ _y_2 0.5)) (< _y (+ _y_2 -0.5))) (or (> _z (+ _z_2 0.5)) (< _z (+ _z_2 -0.5))))
        (`/Engine/EditorBlueprintResources/StandardMacros.DoOnce` false :!label _label
          (:`Completed`
            (`self.ReturnToInitialPosition`)))))))

(event `PlayDisolveAnimation`
  (`SceneComponent.SetVisibility` (`self.TextRender`) false false)
  (bind (_direction _newtrack_0) (`Timeline|Timeline_0` :!via `PlayFromStart`)
    (:`Update`
      (`MaterialInstanceDynamic.SetScalarParameterValue` (`self.MaterialInstance`) "Fade" _newtrack_0))
    (:`Finished`
      (bind _asgm_main (cast `/Game/Blueprints/GM_Main` (`GameplayStatics.GetGameMode`)))
      (`/Game/Blueprints/GM_Main.Action card chosen` _asgm_main (`self.Card`)))))

(event `ResetReturnToLoc`
  (goto _label :!via `Reset`))

(fn `UserConstructionScript`
  (bind _wrapedtext (`self.WrapText` (`.Description_5_28664E6049D95DB37A53C4B70C73F96D` (break `/Game/Datas/F_Card` (`self.Card`))) (`self.Characters per line`)))
  (`TextRenderComponent.K2_SetText` (`self.TextRender`) _wrapedtext)
  (bind _returnvalue (`PrimitiveComponent.CreateDynamicMaterialInstance` (`self.PaperSprite`) 0 "/Game/Materials/DisolveMatTest_Inst.DisolveMatTest_Inst" "None"))
  (set `self.MaterialInstance` _returnvalue))

(fn `WrapText`
  (params (Text :type Text) (`Characters per line` :type Integer))
  (returns (WrapedText :type Text))
  (locals (FinalText :type Text) (CharacterCount :type Integer))
  (set `local.CharacterCount` 0)
  (for _array_element (`KismetStringLibrary.ParseIntoArray` (`KismetTextLibrary.Conv_TextToString` Text))
    (bind _output_get (set `local.CharacterCount` (+ (`KismetStringLibrary.Len` _array_element) (`local.CharacterCount`))))
    (if (> _output_get `Characters per line`)
      (set `local.FinalText` (`|FormatText` "{0}<br> {1}" (`local.FinalText`) _array_element))
      (set `local.CharacterCount` 0)
      (else
        (set `local.FinalText` (`|FormatText` "{0} {1}" (`local.FinalText`) _array_element)))))
  (return (`local.FinalText`)))