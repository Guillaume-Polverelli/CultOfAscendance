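; PC_Main is a player controller for a card game that sets up mouse input and lets the player signal readiness.
; BeginPlay shows the cursor and applies Game and UI input with the mouse locked to the viewport.
; Pressing E calls GameReady on GM_Main through a direct game mode cast.
; The situation and action card drawn events are empty, with their HUD_Main forwarding logic left disconnected.
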(event `self.ReceiveBeginPlay`
  (set `self.bShowMouseCursor` true)
  (`WidgetBlueprintLibrary.SetInputMode_GameAndUIEx` self null "LockAlways" false))

(event `Key|E`
  (params (Key :type "Key Structure"))
  (:`Pressed`
    (bind _asgm_main (cast `/Game/Blueprints/GM_Main` (`GameplayStatics.GetGameMode`)))
    (`/Game/Blueprints/GM_Main.Game Ready` _asgm_main)))

(event `Situation Card Drawn`
  (params (Card :type "/Game/Datas/F_Card Structure")))

(event `Action Cards Drawn`
  (params (Cards :type "Array of /Game/Datas/F_Card Structure")))

(fn `UserConstructionScript`)